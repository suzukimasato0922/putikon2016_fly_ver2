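; Blue trap actor that charges over time and fires a mosquito-killing spray from its own location when NumPad 4 is pressed.
; Tick raises the blue tint of a dynamic material until full, then switches to a bright blue glow and sets a ready flag.
; A press while ready resets tint and charge, spawns the spray hit-detection and effect actors, and plays a spray sound.
; The charge advances per frame, independent of delta time.
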(event EventBeginPlay
  (Input|EnableInput (Game|GetPlayerController 0))
  (bind _returnvalue (Rendering|Material|CreateDynamicMaterialInstance (Variables|Debug|GetStaticMeshComponent) 0 "/Game/大山亮/Trap/TrappBLUE_MAT.TrappBLUE_MAT" :!class /Script/Engine.PrimitiveComponent))
  (Variables|Default|SetDynamicColor _returnvalue))

(event Collision|EventActorBeginOverlap
  (params (OtherActor :type Actor%20Object%20Reference)))

(event EventTick
  (params (DeltaSeconds :type Float%20%28single-precision%29))
  (bind _returnvalue (Rendering|Material|GetVectorParameterValue (Variables|Default|GetDynamicColor) "Base Color Tint" :!class /Script/Engine.MaterialInstanceDynamic))
  (if (< (.z (Math|Conversions|ToVector(LinearColor) _returnvalue)) 1.0)
    (bind _output_get (Variables|Default|Setadd (+ (stale _output_get) 0.0018)))
    (Rendering|Material|SetVectorParameterValue (Variables|Default|GetDynamicColor) "Base Color Tint" (Utilities|Struct|MakeLinearColor 0.0 0.0 (Variables|Default|Getadd) 0.0) :!class /Script/Engine.MaterialInstanceDynamic)
    (else
      (Rendering|Material|SetVectorParameterValue (Variables|Default|GetDynamicColor) "Base Color Tint" (Utilities|Struct|MakeLinearColor 1.0 1.0 1e+02 0.0) :!class /Script/Engine.MaterialInstanceDynamic)
      (Variables|Default|Setok_flg true))))

(event Input|KeyboardEvents|NumPadFour
  (params (Key :type Key%20Structure :default "AnyKey"))
  (bind _returnvalue (Transformation|GetActorTransform))
  (:Pressed
    (if (Variables|Default|Getok_flg)
      (Rendering|Material|SetVectorParameterValue (Variables|Default|GetDynamicColor) "Base Color Tint" (Utilities|Struct|MakeLinearColor 0.0 0.0 0.0 0.0) :!class /Script/Engine.MaterialInstanceDynamic)
      (Variables|Default|Setadd 0.0)
      (Variables|Default|Setok_flg false)
      ;[1 1 1] スプレーと蚊を殺すブロックを配置
      (Game|SpawnActorfromClass "/Game/大山亮/Spray_Hithantei_BP.Spray_Hithantei_BP_C" _returnvalue "Undefined" 0 0)
      (Game|SpawnActorfromClass "/Game/大山亮/SprayEffect_Blueprint.SprayEffect_Blueprint_C" _returnvalue "Undefined" 0 0)
      (Audio|SpawnSound2D "/Game/大山亮/Sounds/スプレー音２.スプレー音２"))))

(fn ConstructionScript
  (Rendering|Material|CreateDynamicMaterialInstance (Variables|Debug|GetStaticMeshComponent) 0 0 :!class /Script/Engine.PrimitiveComponent))